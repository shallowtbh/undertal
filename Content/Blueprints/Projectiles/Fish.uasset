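; Fish projectile that travels out and back along the world Y axis, damaging any Soul_BP it touches.
; Move plays a MoveUp timeline, then MoveDown with its value negated, and destroys the actor when the second finishes.
; Each timeline update adds the curve value to the current Y, so displacement accumulates per update.
; Tick polls the Capsule's overlapping actors and calls TookDamage on Soul_BP, so damage repeats every frame of overlap.
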(event Custom|Move
  (bind _returnvalue (Transformation|GetActorLocation))
  (bind _returnvalue_2 (Transformation|GetActorLocation))
  (bind _moveup (Timeline|MoveUp Play)
    (:Update
      (Transformation|SetActorLocation (Math|Vector|MakeVector (.x _returnvalue_2) (+ _moveup (.y _returnvalue_2)) (.z _returnvalue_2)) false false))
    (:Finished
      (bind _movedown (Timeline|MoveDown Play)
        (:Update
          (Transformation|SetActorLocation (Math|Vector|MakeVector (.x _returnvalue) (+ (* _movedown -1.0) (.y _returnvalue)) (.z _returnvalue)) false false))
        (:Finished
          (Actor|DestroyActor))))))

(event EventTick
  (params (DeltaSeconds :type Float%20%28single-precision%29))
  (for _array_element (Collision|GetOverlappingActors (Variables|Default|GetCapsule) 0 :!class /Script/Engine.PrimitiveComponent)
    (bind _assoul_bp (Utilities|Casting|CastToSoul_BP _array_element))
    (Default|TookDamage _assoul_bp (Variables|Default|GetDamage))))

(fn ConstructionScript)