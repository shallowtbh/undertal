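; Soul Blueprint that handles damage for a three-member party of Kris, Susie and Ralsei.
; TookDamage is gated by an invincibility flag and lowers the health of each member still above zero.
; Kris takes the exact damage, while Susie and Ralsei each get a random offset.
; A delay then clears the flag, with debug prints along the way.
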(event Custom|TookDamage
  (params (Damage :type Integer))
  (if (not (Variables|Default|GetInvincibilityFrames))
    (Variables|Default|SetInvincibilityFrames true)
    (if (> (Variables|Default|GetKrisHealth) 0)
      (Variables|Default|SetKrisHealth (- (Variables|Default|GetKrisHealth) Damage)))
    (if (> (Variables|Default|GetSusieHealth) 0)
      (Variables|Default|SetSusieHealth (- (Variables|Default|GetSusieHealth) (+ (Math|Random|RandomIntegerinRange 5 -5) Damage))))
    (if (> (Variables|Default|GetRalseiHealth) 0)
      (Variables|Default|SetRalseiHealth (- (Variables|Default|GetRalseiHealth) (+ Damage (Math|Random|RandomIntegerinRange 5 0))))
      (Development|PrintString "Hello"))
    (Utilities|FlowControl|Delay 2.5)
    (Development|PrintString "no more invincibility")
    (Variables|Default|SetInvincibilityFrames false)))

(fn ConstructionScript)